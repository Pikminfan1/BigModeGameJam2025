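; Player component that tracks separate XP and levels for five skills: throw, jump, speed, revolver and kick.
; Each AddXP function adds to that skill's total, then loops to subtract the threshold, allowing several level-ups with leftover XP carried over.
; Every level-up fires both a general and a skill-specific OnLevelUp call.
; A helper computes a power-curve XP requirement from base, level and exponent.
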(event `LevelUpThrow`)

(fn `AddXP_Jump`
  (params (XPAmount :type Integer))
  (set `self.CurrentXP_Jump` (+ XPAmount (`self.CurrentXP_Jump`)))
  (`self.CheckLevelUp_Jump`))

(fn `AddXP_Kick`
  (params (XPAmount :type Integer))
  (set `self.CurrentXP_Kick` (+ XPAmount (`self.CurrentXP_Kick`)))
  (`self.CheckLevelUp_Kick`))

(fn `AddXP_Revolver`
  (params (XPAmount :type Integer))
  (set `self.CurrentXP_Revolver` (+ XPAmount (`self.CurrentXP_Revolver`)))
  (`self.CheckLevelUp_Revolver`))

(fn `AddXP_Speed`
  (params (XPAmount :type Integer))
  (set `self.CurrentXP_Speed` (+ XPAmount (`self.CurrentXP_Speed`)))
  (`self.CheckLevelUp_Speed`))

(fn `AddXP_Throw`
  (params (XPAmount :type Integer))
  (set `self.CurrentXP_Throw` (+ XPAmount (`self.CurrentXP_Throw`)))
  (`self.CheckLevelUp_Throw`))

(fn `CheckLevelUp_Jump`
  (bind _currentxp_jump (`self.CurrentXP_Jump`))
  (bind _xptonextlevel_jump (`self.XPToNextLevel_Jump`))
  (while (>= _currentxp_jump _xptonextlevel_jump)
    (set `self.CurrentXP_Jump` (- _currentxp_jump _xptonextlevel_jump))
    (`/Engine/EditorBlueprintResources/StandardMacros.IncrementInt` (`self.JumpLevel`)
      (:`  `
        (`self.OnLevelUp`)
        (`self.OnLevelUp_Jump`)))))

(fn `CheckLevelUp_Kick`
  (bind _currentxp_kick (`self.CurrentXP_Kick`))
  (bind _xptonextlevel_kick (`self.XPToNextLevel_Kick`))
  (while (>= _currentxp_kick _xptonextlevel_kick)
    (set `self.CurrentXP_Kick` (- _currentxp_kick _xptonextlevel_kick))
    (`/Engine/EditorBlueprintResources/StandardMacros.IncrementInt` (`self.KickLevel`)
      (:`  `
        (`self.OnLevelUp`)
        (`self.OnLevelUp_Kick`)))))

(fn `CheckLevelUp_Revolver`
  (bind _currentxp_revolver (`self.CurrentXP_Revolver`))
  (bind _xptonextlevel_revolver (`self.XPToNextLevel_Revolver`))
  (while (>= _currentxp_revolver _xptonextlevel_revolver)
    (set `self.CurrentXP_Revolver` (- _currentxp_revolver _xptonextlevel_revolver))
    (`/Engine/EditorBlueprintResources/StandardMacros.IncrementInt` (`self.RevolverShotLevel`)
      (:`  `
        (`self.OnLevelUp`)
        (`self.OnLevelUp_Revolver`)))))

(fn `CheckLevelUp_Speed`
  (bind _xptonextlevel_speed (`self.XPToNextLevel_Speed`))
  (bind _currentxp_speed (`self.CurrentXP_Speed`))
  (while (>= _currentxp_speed _xptonextlevel_speed)
    (set `self.CurrentXP_Speed` (- _currentxp_speed _xptonextlevel_speed))
    (`/Engine/EditorBlueprintResources/StandardMacros.IncrementInt` (`self.SpeedLevel`)
      (:`  `
        (`self.OnLevelUp`)
        (`self.OnLevelUp_Speed`)))))

(fn `CheckLevelUp_Throw`
  (bind _currentxp_throw (`self.CurrentXP_Throw`))
  (bind _xptonextlevel_throw (`self.XPToNextLevel_Throw`))
  (while (>= _currentxp_throw _xptonextlevel_throw)
    (set `self.CurrentXP_Throw` (- _currentxp_throw _xptonextlevel_throw))
    (`/Engine/EditorBlueprintResources/StandardMacros.IncrementInt` (`self.ThrowLevel`)
      (:`  `
        (`self.OnLevelUp`)
        (`self.OnLevelUp_Throw`)))))

(fn `XPToNextLevel`
  (params (BaseXP :type Integer) (Level :type Integer) (XPExponent :type "Float (double-precision)"))
  (returns (XPToNextLevel :type Integer))
  (return (`KismetMathLibrary.FTrunc` (* BaseXP (`KismetMathLibrary.MultiplyMultiply_FloatFloat` (`KismetMathLibrary.Conv_IntToDouble` Level) XPExponent)))))