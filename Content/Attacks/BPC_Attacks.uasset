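; BPC_Attacks is an attack component that gives its owner projectile and line-trace attacks.
; Projectile attacks spawn BP_Projectile_Base toward a target, then on impact apply damage, report it to AI damage sense and signal attack end.
; Line-trace attacks hit pawns or destructibles with debug drawing, apply damage through the same message, and report it only for Throw damage.
; XP award calls exist but are disconnected.
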(event `Projectile Attack`
  (params (SpawnTransform :type "Transform Structure") (Target :type "Actor Object Reference") (DamageInfo :type "/Game/Blueprints/DamageSystem/S_DamageInfo Structure"))
  (bind _returnvalue (`|SpawnActorFromClass` "/Game/Projectiles/BP_Projectile_Base.BP_Projectile_Base_C" SpawnTransform "Undefined" "MultiplyWithRoot" (`self.GetOwner`) 500.0 0.0 Target false (struct) null))
  (add `/Game/Projectiles/BP_Projectile_Base.OnProjectileImpact` _returnvalue (delegate `OnProjectileHit`)))

(event `OnProjectileHit`
  (params (OtherActor :type "Actor Object Reference") (Hit :type "HitResult Structure"))
  (bind _returnvalue (`self.GetOwner`))
  (message `/Game/Blueprints/DamageSystem/BPI_Damagable.TakeDamageActor` OtherActor (stale `Projectile Attack` DamageInfo) _returnvalue (struct))
  (`AISense_Damage.ReportDamageEvent` OtherActor _returnvalue (`.Amount_2_E8490888454D73137FB8D69A6C4624D8` (break `/Game/Blueprints/DamageSystem/S_DamageInfo` (stale `Projectile Attack` DamageInfo))) (`Actor.K2_GetActorLocation` (`self.GetOwner`)))
  (`self.OnAttackEnded`))

(event `Line Trace Attack (Third Person)`
  (params (Start :type "Vector Structure") (End :type "Vector Structure") (DamageInfo :type "/Game/Blueprints/DamageSystem/S_DamageInfo Structure"))
  (bind (_amount _damagetype) (break `/Game/Blueprints/DamageSystem/S_DamageInfo` DamageInfo))
  (bind _returnvalue (`self.GetOwner`))
  (bind _outhit (`KismetSystemLibrary.LineTraceSingleForObjects` :`Start` Start :`End` End :`ObjectTypes` (`|MakeArray` "ObjectTypeQuery3" "ObjectTypeQuery6" :!type "EObjectTypeQuery Enum") :`DrawDebugType` "ForDuration"))
  (bind (_bblockinghit _binitialoverlap _time _distance _location _impactpoint _normal _impactnormal _physmat _hitactor) (`GameplayStatics.BreakHitResult` _outhit))
  (message `/Game/Blueprints/DamageSystem/BPI_Damagable.TakeDamageActor` _hitactor DamageInfo _returnvalue (struct))
  ; Award XP to Throw, Line Trace or Melee
  (switch `/Game/Blueprints/DamageSystem/E_DamageType` _damagetype
    (:`NewEnumerator5`
      (`AISense_Damage.ReportDamageEvent` _hitactor _returnvalue _amount (`Actor.K2_GetActorLocation` _returnvalue)))))