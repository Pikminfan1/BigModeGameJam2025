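; Game mode for a BigMode Game Jam 2025 game that runs a play timer and reacts to area clears.
; On BeginPlay it resets and starts the timer, which accumulates world delta seconds through a self-calling 0.01s Delay loop, and binds to BP_SpawnManager's area-clear event.
; Clearing one area briefly shows WB_TitleScreen, while clearing the final one stops the timer and shows WB_ScoreScreen.
; Next-area and final-score functions are empty stubs.
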(event `self.ReceiveBeginPlay`
  (`self.Reset Values`)
  (`self.Start Timer`)
  (bind _returnvalue (`GameplayStatics.GetActorOfClass` "/Game/Blueprints/LevelActors/BP_SpawnManager.BP_SpawnManager_C"))
  (`/Engine/EditorBlueprintResources/StandardMacros.IsValid` _returnvalue
    (:`Is Valid`
      (add `/Game/Blueprints/LevelActors/BP_SpawnManager.OnAreaClear` _returnvalue (`|CreateDelegate` :!event `CheckIfChurchClear`)))))

(event `Start Timer`
  ; Timer Controls
  (set `self.TimerActive` true)
  (`self.Update Timer`))

(event `Reset Timer`
  ; Timer Controls
  (set `self.ElapsedTime` 0.0))

(event `Update Timer`
  ; Timer Controls
  (set `self.ElapsedTime` (+ (`GameplayStatics.GetWorldDeltaSeconds`) (`self.ElapsedTime`)))
  (if (`self.TimerActive`)
    (`KismetSystemLibrary.Delay` 0.01)
    (`self.Update Timer`)))

(event `Stop Timer`
  ; Timer Controls
  (set `self.TimerActive` false))

(event `End Game`
  ; On Game End
  ;; Pause
  (`GameplayStatics.SetGamePaused` false)
  (`self.Stop Timer`)
  (bind _returnvalue (`|CreateWidget` "/Game/UI/WB_ScoreScreen.WB_ScoreScreen_C"))
  (`UserWidget.AddToViewport` _returnvalue 0))

(event `CheckIfChurchClear`
  (params (AreaCleared :type "/Game/Blueprints/LevelActors/E_Area Enum" :default "NewEnumerator0"))
  (if (`|EnumEquality` AreaCleared "NewEnumerator5")
    (`self.End Game`)
    (elif (`|EnumEquality` AreaCleared "NewEnumerator1")
      (bind _returnvalue (`|CreateWidget` "/Game/UI/WB_TitleScreen.WB_TitleScreen_C"))
      (`UserWidget.AddToViewport` _returnvalue 0)
      (`KismetSystemLibrary.K2_SetTimerDelegate` (delegate `DestroyScreen`) 5.0))))

(event `DestroyScreen`
  (`Widget.RemoveFromParent` (stale `CheckIfChurchClear` _returnvalue)))

(fn `CalculateFinalScore`)

(fn `GetNextArea`
  (params (CurrentArea :type "/Game/Blueprints/LevelActors/E_Area Enum" :default "NewEnumerator0")))

(fn `Reset Values`
  (set `self.ElapsedTime` 0.0))

(fn `SetDifficulty`
  (params (Difficulty :type "/Game/Blueprints/LevelActors/E_Difficulty Enum" :default "NewEnumerator0"))
  (set `self.CurrentDifficulty` Difficulty))

(fn `UserConstructionScript`)