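; BP_Enemy_Ranged is a child enemy character that fights at range with a pistol.
; On BeginPlay it spawns the pistol onto a hand socket; unequipping plays a sheath montage whose notify destroys it.
; Attacks play a montage whose notify has the attacks component line-trace damage from weapon to target.
; It also sets starting health, maps speed states to walk speeds and reports ideal ranges, while both health getters return zero.
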(event `self.ReceiveBeginPlay`
  (`parent.ReceiveBeginPlay`)
  (`self.EquipWeapon`))

(event `/Game/Blueprints/AI/EnemyAI/BPI_EnemyAI.EquipWeapon`
  (bind _returnvalue (`|SpawnActorFromClass` "/Game/Weapons/BP_Weapon_Pistol.BP_Weapon_Pistol_C" (`KismetMathLibrary.MakeTransform` (0.0 0.0 0.0)) "Undefined" "MultiplyWithRoot" null null))
  (bind _output_get (set `self.WeaponActor` _returnvalue))
  (`self.K2_AttachToComponent` _output_get (`self.Mesh`) "PistolSocket_r" "KeepRelative" "KeepRelative" "KeepRelative" true)
  (set `self.IsWieldingWeapon` true)
  (`self.OnWeaponEquipped`))

(event `/Game/Blueprints/AI/EnemyAI/BPI_EnemyAI.UnEquipWeapon`
  (bind _notifyname (`|PlayMontage` (`self.Mesh`) (`self.SheathMeleeWeaponMontage`))
    (:`OnCompleted`
      (`self.OnWeaponUnequipped` :!label _label))
    (:`OnInterrupted`
      (goto _label))
    (:`OnNotifyBegin`
      (switch `name` _notifyname
        (:`SheathWeapon`
          (`self.K2_DestroyActor` (`self.WeaponActor`))
          (set `self.IsWieldingWeapon` false))))))

(event `/Game/Blueprints/AI/EnemyAI/BPI_EnemyAI.Attack`
  (params (AttackTarget :type "Actor Object Reference"))
  ; Fire Gun
  (bind _notifyname (`|PlayMontage` (`self.Mesh`) (`self.AttackMontage`))
    (:`OnCompleted`
      (`self.AttackEnd` AttackTarget :!label _label_2))
    (:`OnInterrupted`
      (goto _label_2))
    (:`OnNotifyBegin`
      (switch `name` _notifyname
        (:`Fire`
          (`/Game/Attacks/BPC_Attacks.Line Trace Attack (Third Person)` (`self.BPC_Attacks`) (`self.K2_GetActorLocation` (`self.WeaponActor`)) (`self.K2_GetActorLocation` AttackTarget) (make `/Game/Blueprints/DamageSystem/S_DamageInfo` 15.0 "NewEnumerator2")))))))

(fn `GetHealth`
  (returns (CurrentHealth :type "Float (double-precision)"))
  (return 0.0))

(fn `GetIdealRange`
  (returns (AttackRadius :type "Float (double-precision)") (DefendRadius :type "Float (double-precision)"))
  (return 600.0 600.0))

(fn `GetMaximumHealth`
  (returns (MaxHealth :type "Float (double-precision)"))
  (return 0.0))

(fn `SetMovementSpeed`
  (params (Speed :type "/Game/Blueprints/AI/EnemyAI/Enums/E_MovementSpeed Enum" :default "NewEnumerator0"))
  (returns (SpeedValue :type "Float (double-precision)"))
  (bind _output_get (set `CharacterMovementComponent.MaxWalkSpeed` (select `/Game/Blueprints/AI/EnemyAI/Enums/E_MovementSpeed` Speed :`NewEnumerator1` 200.0 :`NewEnumerator2` 300.0 :`NewEnumerator3` 500.0) (`self.CharacterMovement`)))
  (return _output_get))

(fn `UserConstructionScript`
  (set `/Game/Blueprints/DamageSystem/BPC_DamageSystem.Health` 100.0 (`self.BPC_DamageSystem`))
  (set `/Game/Blueprints/DamageSystem/BPC_DamageSystem.MaxHealth` 100.0 (`self.BPC_DamageSystem`))
  (`parent.UserConstructionScript`))