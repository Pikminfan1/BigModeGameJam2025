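; Base enemy character that delegates health, damage and attack tokens to BPCDamageSystem and drives its AI controller's states.
; Attacks reserve tokens from the target, returning them on attack end or death.
; Hits freeze the AI during a montage; kicks ragdoll the enemy until a timer restores walking.
; Death awards XP by enemy type, ragdolls and delays destruction; a projectile-arc launch handles smart-link jumps, while blocking is stubbed.
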(event `self.ReceiveBeginPlay`
  ; Initialize Widgets, Bind On Death and Hit response, initialize widgets
  (bind _asbp_enemy_aicontroller (cast `/Game/Blueprints/AI/EnemyAI/EnemyAIControllers/BP_EnemyAIController` (`AIBlueprintHelperLibrary.GetAIController` self)))
  (set `self.BP Enemy AIController` _asbp_enemy_aicontroller)
  (`KismetSystemLibrary.Delay` 0.2)
  (bind _returnvalue (`|CreateWidget` "/Game/Blueprints/DamageSystem/W_Healthbar.W_Healthbar_C" null self))
  (`WidgetComponent.SetWidget` (`self.Health Bar`) _returnvalue)
  (add `/Game/Blueprints/DamageSystem/BPC_DamageSystem.OnDeath` (`self.BPC_DamageSystem`) (`|CreateDelegate` :!event `Die`))
  (add `/Game/Blueprints/DamageSystem/BPC_DamageSystem.OnDamageResponse` (`self.BPC_DamageSystem`) (`|CreateDelegate` :!event `HitResponse`))
  (bind _asbp_hybrid_character (cast `/Game/HybridPlayerController/BP_HybridCharacter` (`GameplayStatics.GetPlayerCharacter` 0)))
  (set `self.Player Character_Ref` _asbp_hybrid_character))

(event `/Game/Blueprints/AI/EnemyAI/BPI_EnemyAI.JumpToDestination`
  (params (Destination :type "Vector Structure"))
  ; Event to help ai navigate smart links using a jump. Jump assist gives them the boost they need to clear most jumps
  (bind _outlaunchvelocity (`GameplayStatics.SuggestProjectileVelocity_CustomArc` (`self.K2_GetActorLocation`) (`KismetMathLibrary.MakeVector` Destination_X Destination_Y (+ Destination_Z (`self.JumpAssist`)))))
  (`self.LaunchCharacter` _outlaunchvelocity true true))

(event `Die`
  (bind _mesh (`self.Mesh`))
  (bind _reservedattacktokens (`self.ReservedAttackTokens`))
  (bind _basejumpxpreward (`self.BaseJumpXPReward`))
  (bind _player_character_ref (`self.Player Character_Ref`))
  ; Event For Enemies Dying. Will not delete actor (want to implement revive) Implement function to actually destroy actor when the time is right. Tokens they still possess are returned
  (`|ExecutionSequence`
    (:`then_0`
      (switch `/Game/Blueprints/E_EnemyBonusType` (`self.EnemyType`) :!label _label
        (:`NewEnumerator1`
          (`/Game/HybridPlayerController/BPI_PlayerInterface.AwardXP` _player_character_ref _basejumpxpreward "NewEnumerator1"))
        (:`NewEnumerator2`
          (`/Game/HybridPlayerController/BPI_PlayerInterface.AwardXP` _player_character_ref _basejumpxpreward "NewEnumerator2"))))
    (:`then_1`
      (`AkGameplayStatics.PostEvent` "/Game/WwiseAudio/Events/Default_Work_Unit/EnemyDeath.EnemyDeath" self 17152)
      (`PrimitiveComponent.SetSimulatePhysics` _mesh true)
      (`PrimitiveComponent.SetCollisionEnabled` (`self.CapsuleComponent`) "NoCollision")
      (`PrimitiveComponent.SetCollisionEnabled` _mesh "QueryAndPhysics")
      (`BrainComponent.StopLogic` (`AIController.BrainComponent` (`self.BP Enemy AIController`)) "")
      (`/Game/Blueprints/AI/EnemyAI/EnemyAIControllers/BP_EnemyAIController.SetStateAsDead` (`self.BP Enemy AIController`))
      (`self.OnEnemyDied`)
      (`SceneComponent.SetVisibility` (`self.Health Bar`) false true)
      (bind _keys (`BlueprintMapLibrary.Map_Keys` _reservedattacktokens))
      (for _array_element _keys
        (message `/Game/Blueprints/DamageSystem/BPI_Damagable.ReturnAttackToken` _array_element (`BlueprintMapLibrary.Map_Find` _reservedattacktokens _array_element))
        (`PrimitiveComponent.SetCollisionEnabled` (`self.CapsuleComponent`) "NoCollision")
        (goto _label)))
    (:`then_2`
      (`KismetSystemLibrary.Delay` 10.0)
      (`self.K2_DestroyActor`))))

(event `HitResponse`
  (params (DamageResponse :type "/Game/Blueprints/DamageSystem/E_DamageResponse Enum" :default "NewEnumerator0") (DamageCauser :type "Actor Object Reference"))
  (bind _bp_enemy_aicontroller (`self.BP Enemy AIController`))
  ; Handle What happens when the actor is hit by an attack
  (`MovementComponent.StopMovementImmediately` (`self.CharacterMovement`))
  (`/Game/Blueprints/AI/EnemyAI/EnemyAIControllers/BP_EnemyAIController.SetStateAsFrozen` (`self.BP Enemy AIController`))
  (`|PlayMontage` (`self.Mesh`) (`self.Hit Montage`) (`self.Hit Montage Play Rate`) (`self.Hit Montage Start Pos`)
    (:`OnCompleted`
      _)
    (:`OnInterrupted`
      _))
  (`/Engine/EditorBlueprintResources/StandardMacros.IsValid` _bp_enemy_aicontroller
    (:`Is Valid`
      (`/Game/Blueprints/AI/EnemyAI/EnemyAIControllers/BP_EnemyAIController.SetStateAsAttacking` _bp_enemy_aicontroller DamageCauser true))))

(event `/Game/Blueprints/DamageSystem/BPI_Damagable.ReturnAttackToken`
  (params (Amount :type Integer))
  ; Attack Token System
  ; -Each Actor that has a DamageSystem component can make use of the token system (Including enemies amongst themselves if we wish)
  ; -Tokens are requested from the attack target. There are a limited amount of tokens to distribute, and attacks have the ability to "cost" more tokens if need be
  ; -Tokens Are returned when attacks are completed, or interupted in anyway (Enemy takes hit, dies, etc)
  (`/Game/Blueprints/DamageSystem/BPC_DamageSystem.ReturnAttackToken` (`self.BPC_DamageSystem`) Amount))

(event `/Game/Blueprints/AI/EnemyAI/BPI_EnemyAI.StoreAttackTokens`
  (params (AttackTarget :type "Actor Object Reference") (Amount :type Integer))
  (bind (_value _returnvalue) (`BlueprintMapLibrary.Map_Find` (`self.ReservedAttackTokens`) AttackTarget))
  ; Attack Token System
  ; -Each Actor that has a DamageSystem component can make use of the token system (Including enemies amongst themselves if we wish)
  ; -Tokens are requested from the attack target. There are a limited amount of tokens to distribute, and attacks have the ability to "cost" more tokens if need be
  ; -Tokens Are returned when attacks are completed, or interupted in anyway (Enemy takes hit, dies, etc)
  (`BlueprintMapLibrary.Map_Add` (`self.ReservedAttackTokens`) AttackTarget (`KismetMathLibrary.SelectInt` (+ Amount _value) Amount _returnvalue)))

(event `/Game/Blueprints/AI/EnemyAI/BPI_EnemyAI.AttackEnd`
  (params (AttackTarget :type "Actor Object Reference"))
  (bind _tokensusedincurrentattack (`self.TokensUsedInCurrentAttack`))
  ; Attack Token System
  ; -Each Actor that has a DamageSystem component can make use of the token system (Including enemies amongst themselves if we wish)
  ; -Tokens are requested from the attack target. There are a limited amount of tokens to distribute, and attacks have the ability to "cost" more tokens if need be
  ; -Tokens Are returned when attacks are completed, or interupted in anyway (Enemy takes hit, dies, etc)
  (message `/Game/Blueprints/DamageSystem/BPI_Damagable.ReturnAttackToken` AttackTarget _tokensusedincurrentattack)
  (`/Game/Blueprints/AI/EnemyAI/BPI_EnemyAI.StoreAttackTokens` AttackTarget (* _tokensusedincurrentattack -1))
  (set `self.Attacking` false)
  (`self.OnAttackEnd`))

(event `/Game/Blueprints/AI/EnemyAI/BPI_EnemyAI.Attack`
  (params (AttackTarget :type "Actor Object Reference"))
  ; Attack Token System
  ; -Each Actor that has a DamageSystem component can make use of the token system (Including enemies amongst themselves if we wish)
  ; -Tokens are requested from the attack target. There are a limited amount of tokens to distribute, and attacks have the ability to "cost" more tokens if need be
  ; -Tokens Are returned when attacks are completed, or interupted in anyway (Enemy takes hit, dies, etc)
  (set `self.Attacking` true))

(event `LandEventSetup`
  ; Land Event
  (bind _returnvalue (`KismetSystemLibrary.K2_SetTimerDelegate` (delegate `LandEventHandle`) 5.0))
  (set `self.LandingTimerHandle` _returnvalue))

(event `LandEventHandle`
  (bind _capsulecomponent (`self.CapsuleComponent`))
  (bind _mesh (`self.Mesh`))
  ; Land Event
  (`PrimitiveComponent.SetSimulatePhysics` _mesh false)
  ;; Revisit this
  (`PrimitiveComponent.SetCollisionEnabled` (`self.CapsuleComponent`) "QueryOnly")
  (`PrimitiveComponent.SetCollisionEnabled` _mesh "NoCollision")
  (set `PrimitiveComponent.bGenerateOverlapEvents` false _mesh)
  (`SceneComponent.K2_AttachToComponent` _mesh _capsulecomponent "None" "SnapToTarget" "KeepRelative" "KeepRelative" true)
  (`SceneComponent.K2_SetWorldLocation` _capsulecomponent (`SceneComponent.GetSocketLocation` _mesh "pelvis") false true)
  (`SceneComponent.K2_SetRelativeTransform` _mesh (`KismetMathLibrary.MakeTransform` (0.0 0.0 -80.0) (struct :`Yaw` -90.0)) false false)
  (`CharacterMovementComponent.SetMovementMode` (`self.CharacterMovement`) "MOVE_Walking" 0))

(event `/Game/Blueprints/DamageSystem/BPI_Damagable.SetActorCurrentHealth`
  (params (BaseCurrentHealth :type "Float (double-precision)"))
  (set `/Game/Blueprints/DamageSystem/BPC_DamageSystem.Health` BaseCurrentHealth (`self.BPC_DamageSystem`)))

(event `/Game/Blueprints/DamageSystem/BPI_Damagable.SetActorCurrentMaxHealth`
  (params (BaseMaxHealth :type "Float (double-precision)"))
  (set `/Game/Blueprints/DamageSystem/BPC_DamageSystem.MaxHealth` BaseMaxHealth (`self.BPC_DamageSystem`)))

(event `Set Parent Spawner`
  (params (`Parent Spawner` :type "/Game/Blueprints/LevelActors/BP_Spawner Object Reference"))
  (set `self.ParentSpawner` `Parent Spawner`))

(fn `AttackStart`
  (params (AttackTarget :type "Actor Object Reference") (TokensNeeded :type Integer))
  (returns (Success :type Boolean))
  (bind _success (message `/Game/Blueprints/DamageSystem/BPI_Damagable.ReserveAttackToken` AttackTarget TokensNeeded))
  (if _success
    (`/Game/Blueprints/AI/EnemyAI/BPI_EnemyAI.StoreAttackTokens` AttackTarget TokensNeeded)
    (set `self.TokensUsedInCurrentAttack` TokensNeeded)
    (return true)
    (else
      (return false))))

(fn `AttemptBlock`)

(fn `GetActorCurrentHealth`
  (returns (Health :type "Float (double-precision)"))
  (return (`/Game/Blueprints/DamageSystem/BPC_DamageSystem.Health` (`self.BPC_DamageSystem`))))

(fn `GetActorMaxHealth`
  (returns (MaxHealth :type "Float (double-precision)"))
  (return (`/Game/Blueprints/DamageSystem/BPC_DamageSystem.MaxHealth` (`self.BPC_DamageSystem`))))

(fn `GetIdealRange`
  (returns (AttackRadius :type "Float (double-precision)") (DefendRadius :type "Float (double-precision)"))
  (return 150.0 350.0))

(fn `GetPatrolRoute`
  (returns (PatrolRoute :type "/Game/Blueprints/AI/EnemyAI/BP_PatrolRoute Object Reference"))
  (return (`self.PatrolRoute`)))

(fn `HealActor`
  (params (Amount :type "Float (double-precision)"))
  (returns (NewHealth :type "Float (double-precision)"))
  (bind _newhealth (`/Game/Blueprints/DamageSystem/BPC_DamageSystem.Heal` (`self.BPC_DamageSystem`) Amount))
  (return _newhealth))

(fn `IsAttacking`
  (returns (Attacking :type Boolean))
  (return false))

(fn `IsDead`
  (returns (IsActrorDead :type Boolean))
  (return (`/Game/Blueprints/DamageSystem/BPC_DamageSystem.IsDead` (`self.BPC_DamageSystem`))))

(fn `ReserveAttackToken`
  (params (Amount :type Integer))
  (returns (Success :type Boolean))
  (bind _success (`/Game/Blueprints/DamageSystem/BPC_DamageSystem.ReserveAttackToken` (`self.BPC_DamageSystem`) Amount))
  (return _success))

(fn `SetMovementSpeed`
  (params (Speed :type "/Game/Blueprints/AI/EnemyAI/Enums/E_MovementSpeed Enum" :default "NewEnumerator0"))
  (returns (SpeedValue :type "Float (double-precision)"))
  (bind _output_get (set `CharacterMovementComponent.MaxWalkSpeed` (select `/Game/Blueprints/AI/EnemyAI/Enums/E_MovementSpeed` Speed :`NewEnumerator1` 100.0 :`NewEnumerator2` 300.0 :`NewEnumerator3` 500.0) (`self.CharacterMovement`)))
  (return _output_get))

(fn `TakeDamageActor`
  (params (DamageInfo :type "/Game/Blueprints/DamageSystem/S_DamageInfo Structure") (DamageCauseActor :type "Actor Object Reference") (HitResult :type "HitResult Structure"))
  (returns (WasDamaged :type Boolean))
  (bind _mesh (`self.Mesh`))
  (switch `/Game/Blueprints/DamageSystem/E_DamageType` (`.DamageType_5_29B2026548B8118A5929CB9A0496E3A7` (break `/Game/Blueprints/DamageSystem/S_DamageInfo` DamageInfo))
    (:`NewEnumerator0`
      _)
    (:`NewEnumerator1`
      _)
    (:`NewEnumerator2`
      (message `/Game/HybridPlayerController/BPI_PlayerInterface.AwardXP` DamageCauseActor 3 "NewEnumerator4"))
    (:`NewEnumerator3`
      (message `/Game/HybridPlayerController/BPI_PlayerInterface.AwardXP` DamageCauseActor 20 "NewEnumerator3")
      (`PrimitiveComponent.SetSimulatePhysics` _mesh true)
      (`PrimitiveComponent.SetCollisionEnabled` (`self.CapsuleComponent`) "NoCollision")
      (`PrimitiveComponent.SetCollisionEnabled` _mesh "QueryAndPhysics")
      (`PrimitiveComponent.AddImpulse` (`self.Mesh`) (* (`self.GetActorForwardVector` DamageCauseActor) (30000.0 30000.0 30000.0)) "pelvis" true)
      (set `PrimitiveComponent.bGenerateOverlapEvents` true (`self.Mesh`))
      (`CharacterMovementComponent.DisableMovement` (`self.CharacterMovement`))
      (`self.LandEventSetup`))
    (:`NewEnumerator4`
      _)
    (:`NewEnumerator5`
      (message `/Game/HybridPlayerController/BPI_PlayerInterface.AwardXP` DamageCauseActor 20 "NewEnumerator5")))
  (bind _wasdamaged (`/Game/Blueprints/DamageSystem/BPC_DamageSystem.TakeDamage` (`self.BPC_DamageSystem`) DamageInfo DamageCauseActor))
  (return _wasdamaged))

(fn `UserConstructionScript`)