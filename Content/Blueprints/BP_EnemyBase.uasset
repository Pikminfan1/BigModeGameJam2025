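; Base enemy character that takes damage, reacts to hits, ragdolls on death and jumps smart links with an assisted launch arc.
; BPC_DamageSystem owns health and drives the healthbar widget, death and hit-response events, which set AI controller states.
; Attacks reserve limited tokens from their target, tracked per target and returned on attack end or death.
; Interface-style functions expose health, patrol route, ideal ranges and movement speed presets.
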(event `self.ReceiveBeginPlay`
  ; Initialize Widgets, Bind On Death and Hit response, initialize widgets
  (bind _asbp_enemy_aicontroller (cast `/Game/Blueprints/AI/EnemyAI/BP_EnemyAIController` (`AIBlueprintHelperLibrary.GetAIController` self)))
  (set `self.BP Enemy AIController` _asbp_enemy_aicontroller)
  (`KismetSystemLibrary.Delay` 0.2)
  (bind _returnvalue (`|CreateWidget` "/Game/Blueprints/DamageSystem/W_Healthbar.W_Healthbar_C" null self))
  (`WidgetComponent.SetWidget` (`self.Health Bar`) _returnvalue)
  (add `/Game/Blueprints/DamageSystem/BPC_DamageSystem.OnDeath` (`self.BPC_DamageSystem`) (`|CreateDelegate` :!event `Die`))
  (add `/Game/Blueprints/DamageSystem/BPC_DamageSystem.OnDamageResponse` (`self.BPC_DamageSystem`) (`|CreateDelegate` :!event `HitResponse`)))

(event `/Game/Blueprints/AI/EnemyAI/BPI_EnemyAI.JumpToDestination`
  (params (Destination :type "Vector Structure"))
  ; Event to help ai navigate smart links using a jump. Jump assist gives them the boost they need to clear most jumps
  (bind _outlaunchvelocity (`GameplayStatics.SuggestProjectileVelocity_CustomArc` (`self.K2_GetActorLocation`) (`KismetMathLibrary.MakeVector` Destination_X Destination_Y (+ Destination_Z (`self.JumpAssist`)))))
  (`self.LaunchCharacter` _outlaunchvelocity true true))

(event `Die`
  (bind _mesh (`self.Mesh`))
  (bind _reservedattacktokens (`self.ReservedAttackTokens`))
  ; Event For Enemies Dying. Will not delete actor (want to implement revive) Implement function to actually destroy actor when the time is right. Tokens they still possess are returned
  (`PrimitiveComponent.SetSimulatePhysics` _mesh true)
  (`PrimitiveComponent.SetCollisionEnabled` _mesh "QueryAndPhysics")
  (`BrainComponent.StopLogic` (`AIController.BrainComponent` (`self.BP Enemy AIController`)) "")
  (`/Game/Blueprints/AI/EnemyAI/BP_EnemyAIController.SetStateAsDead` (`self.BP Enemy AIController`))
  (`SceneComponent.SetVisibility` (`self.Health Bar`) false true)
  (bind _keys (`BlueprintMapLibrary.Map_Keys` _reservedattacktokens))
  (for _array_element _keys
    (message `/Game/Blueprints/DamageSystem/BPI_Damagable.ReturnAttackToken` _array_element (`BlueprintMapLibrary.Map_Find` _reservedattacktokens _array_element))))

(event `HitResponse`
  (params (DamageResponse :type "/Game/Blueprints/DamageSystem/E_DamageResponse Enum" :default "NewEnumerator0") (DamageCauser :type "Actor Object Reference"))
  (bind _bp_enemy_aicontroller (`self.BP Enemy AIController`))
  ; Handle What happens when the actor is hit by an attack
  (`MovementComponent.StopMovementImmediately` (`self.CharacterMovement`))
  (`/Game/Blueprints/AI/EnemyAI/BP_EnemyAIController.SetStateAsFrozen` (`self.BP Enemy AIController`))
  (`|PlayMontage` (`self.Mesh`) (`self.Hit Montage`) (`self.Hit Montage Play Rate`) (`self.Hit Montage Start Pos`)
    (:`OnCompleted`
      _)
    (:`OnInterrupted`
      _))
  (`/Engine/EditorBlueprintResources/StandardMacros.IsValid` _bp_enemy_aicontroller
    (:`Is Valid`
      (`/Game/Blueprints/AI/EnemyAI/BP_EnemyAIController.SetStateAsAttacking` _bp_enemy_aicontroller DamageCauser true))))

(event `/Game/Blueprints/DamageSystem/BPI_Damagable.ReturnAttackToken`
  (params (Amount :type Integer))
  ; Attack Token System
  ; -Each Actor that has a DamageSystem component can make use of the token system (Including enemies amongst themselves if we wish)
  ; -Tokens are requested from the attack target. There are a limited amount of tokens to distribute, and attacks have the ability to "cost" more tokens if need be
  ; -Tokens Are returned when attacks are completed, or interupted in anyway (Enemy takes hit, dies, etc)
  (`/Game/Blueprints/DamageSystem/BPC_DamageSystem.ReturnAttackToken` (`self.BPC_DamageSystem`) Amount))

(event `/Game/Blueprints/AI/EnemyAI/BPI_EnemyAI.StoreAttackTokens`
  (params (AttackTarget :type "Actor Object Reference") (Amount :type Integer))
  (bind (_value _returnvalue) (`BlueprintMapLibrary.Map_Find` (`self.ReservedAttackTokens`) AttackTarget))
  ; Attack Token System
  ; -Each Actor that has a DamageSystem component can make use of the token system (Including enemies amongst themselves if we wish)
  ; -Tokens are requested from the attack target. There are a limited amount of tokens to distribute, and attacks have the ability to "cost" more tokens if need be
  ; -Tokens Are returned when attacks are completed, or interupted in anyway (Enemy takes hit, dies, etc)
  (`BlueprintMapLibrary.Map_Add` (`self.ReservedAttackTokens`) AttackTarget (`KismetMathLibrary.SelectInt` (+ Amount _value) Amount _returnvalue)))

(event `/Game/Blueprints/AI/EnemyAI/BPI_EnemyAI.AttackEnd`
  (params (AttackTarget :type "Actor Object Reference"))
  (bind _tokensusedincurrentattack (`self.TokensUsedInCurrentAttack`))
  ; Attack Token System
  ; -Each Actor that has a DamageSystem component can make use of the token system (Including enemies amongst themselves if we wish)
  ; -Tokens are requested from the attack target. There are a limited amount of tokens to distribute, and attacks have the ability to "cost" more tokens if need be
  ; -Tokens Are returned when attacks are completed, or interupted in anyway (Enemy takes hit, dies, etc)
  (message `/Game/Blueprints/DamageSystem/BPI_Damagable.ReturnAttackToken` AttackTarget _tokensusedincurrentattack)
  (`/Game/Blueprints/AI/EnemyAI/BPI_EnemyAI.StoreAttackTokens` AttackTarget (* _tokensusedincurrentattack -1))
  (set `self.Attacking` false)
  (`self.OnAttackEnd`))

(event `/Game/Blueprints/AI/EnemyAI/BPI_EnemyAI.Attack`
  (params (AttackTarget :type "Actor Object Reference"))
  ; Attack Token System
  ; -Each Actor that has a DamageSystem component can make use of the token system (Including enemies amongst themselves if we wish)
  ; -Tokens are requested from the attack target. There are a limited amount of tokens to distribute, and attacks have the ability to "cost" more tokens if need be
  ; -Tokens Are returned when attacks are completed, or interupted in anyway (Enemy takes hit, dies, etc)
  (set `self.Attacking` true))

(fn `AttackStart`
  (params (AttackTarget :type "Actor Object Reference") (TokensNeeded :type Integer))
  (returns (Success :type Boolean))
  (bind _success (message `/Game/Blueprints/DamageSystem/BPI_Damagable.ReserveAttackToken` AttackTarget TokensNeeded))
  (if _success
    (`/Game/Blueprints/AI/EnemyAI/BPI_EnemyAI.StoreAttackTokens` AttackTarget TokensNeeded)
    (set `self.TokensUsedInCurrentAttack` TokensNeeded)
    (return true)
    (else
      (return false))))

(fn `AttemptBlock`)

(fn `GetActorCurrentHealth`
  (returns (Health :type "Float (double-precision)"))
  (return (`/Game/Blueprints/DamageSystem/BPC_DamageSystem.Health` (`self.BPC_DamageSystem`))))

(fn `GetActorMaxHealth`
  (returns (MaxHealth :type "Float (double-precision)"))
  (return (`/Game/Blueprints/DamageSystem/BPC_DamageSystem.MaxHealth` (`self.BPC_DamageSystem`))))

(fn `GetIdealRange`
  (returns (AttackRadius :type "Float (double-precision)") (DefendRadius :type "Float (double-precision)"))
  (return 150.0 350.0))

(fn `GetPatrolRoute`
  (returns (PatrolRoute :type "/Game/Blueprints/AI/EnemyAI/BP_PatrolRoute Object Reference"))
  (return (`self.PatrolRoute`)))

(fn `HealActor`
  (params (Amount :type "Float (double-precision)"))
  (returns (NewHealth :type "Float (double-precision)"))
  (bind _newhealth (`/Game/Blueprints/DamageSystem/BPC_DamageSystem.Heal` (`self.BPC_DamageSystem`) Amount))
  (return _newhealth))

(fn `IsAttacking`
  (returns (Attacking :type Boolean))
  (return false))

(fn `IsDead`
  (returns (IsActrorDead :type Boolean))
  (return (`/Game/Blueprints/DamageSystem/BPC_DamageSystem.IsDead` (`self.BPC_DamageSystem`))))

(fn `ReserveAttackToken`
  (params (Amount :type Integer))
  (returns (Success :type Boolean))
  (bind _success (`/Game/Blueprints/DamageSystem/BPC_DamageSystem.ReserveAttackToken` (`self.BPC_DamageSystem`) Amount))
  (return _success))

(fn `SetMovementSpeed`
  (params (Speed :type "/Game/Blueprints/AI/EnemyAI/Enums/E_MovementSpeed Enum" :default "NewEnumerator0"))
  (returns (SpeedValue :type "Float (double-precision)"))
  (bind _output_get (set `CharacterMovementComponent.MaxWalkSpeed` (select `/Game/Blueprints/AI/EnemyAI/Enums/E_MovementSpeed` Speed :`NewEnumerator1` 100.0 :`NewEnumerator2` 300.0 :`NewEnumerator3` 500.0) (`self.CharacterMovement`)))
  (return _output_get))

(fn `TakeDamageActor`
  (params (DamageInfo :type "/Game/Blueprints/DamageSystem/S_DamageInfo Structure") (DamageCauseActor :type "Actor Object Reference"))
  (returns (WasDamaged :type Boolean))
  (bind _wasdamaged (`/Game/Blueprints/DamageSystem/BPC_DamageSystem.TakeDamage` (`self.BPC_DamageSystem`) DamageInfo DamageCauseActor))
  (return _wasdamaged))

(fn `UserConstructionScript`)