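; Melee enemy character, child of a parent enemy class, that attacks, draws and sheathes a broom weapon, blocks, and supplies ideal attack and defend ranges.
; Montage notifies time the forward sphere-trace damage, swing sound, and spawning or destroying of the socketed weapon.
; Blocking sets a flag on the damage system component, whose OnBlocked event switches to a hit-reaction montage, with a state check preventing that interruption from ending the block.
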(event `self.ReceiveBeginPlay`
  (`parent.ReceiveBeginPlay`))

(event `/Game/Blueprints/AI/EnemyAI/BPI_EnemyAI.Attack`
  (params (AttackTarget :type "Actor Object Reference"))
  (bind _returnvalue (`self.K2_GetActorLocation`))
  (`parent.Attack` AttackTarget)
  ; Can add IsInteruptable checks after Attack end and play montage to give I frames
  (bind _notifyname (`|PlayMontage` (`self.Mesh`) (`self.AttackMontage`))
    (:`OnCompleted`
      (`self.AttackEnd` AttackTarget :!label _label))
    (:`OnInterrupted`
      (goto _label))
    (:`OnNotifyBegin`
      (switch `name` _notifyname
        (:`MeleeWeaponHit`
          ; Attack Logic
          (bind (_outhit _returnvalue_2) (`KismetSystemLibrary.SphereTraceSingleForObjects` _returnvalue (+ _returnvalue (* (`self.GetActorForwardVector`) (`self.MeleeRange`))) (`self.MeleeRadius`) (`|MakeArray` "ObjectTypeQuery3" :!type "EObjectTypeQuery Enum") false (`|MakeArray` (`self.WeaponActor`) null :!type "Actor Object Reference") "ForDuration"))
          (if _returnvalue_2
            (message `/Game/Blueprints/DamageSystem/BPI_Damagable.TakeDamageActor` (`.HitActor` (`GameplayStatics.BreakHitResult` _outhit)) (make `/Game/Blueprints/DamageSystem/S_DamageInfo` (`self.BaseDamage`) "NewEnumerator1") self (struct))))
        (:`SwingSound`
          (`AkGameplayStatics.PostEvent` "/Game/WwiseAudio/Events/SFX/Woosh.Woosh" self))))))

(event `/Game/Blueprints/AI/EnemyAI/BPI_EnemyAI.UnEquipWeapon`
  (bind _notifyname (`|PlayMontage` (`self.Mesh`) (`self.SheathMeleeWeaponMontage`))
    (:`OnCompleted`
      (`self.OnWeaponUnequipped`))
    (:`OnNotifyBegin`
      (switch `name` _notifyname
        (:`SheathWeapon`
          (`self.K2_DestroyActor` (`self.WeaponActor`))
          (set `self.IsWieldingWeapon` false))))))

(event `/Game/Blueprints/AI/EnemyAI/BPI_EnemyAI.EquipWeapon`
  (bind _notifyname (`|PlayMontage` (`self.Mesh`) (`self.DrawMeleeWeaponMontage`))
    (:`OnCompleted`
      (`self.OnWeaponEquipped`))
    (:`OnNotifyBegin`
      (switch `name` _notifyname
        (:`WieldWeapon`
          (bind _returnvalue (`|SpawnActorFromClass` "/Game/Weapons/BP_Weapon_Broom.BP_Weapon_Broom_C" (`self.GetTransform`) "Undefined" "MultiplyWithRoot" null null))
          (set `self.WeaponActor` _returnvalue)
          (`self.K2_AttachToComponent` (`self.WeaponActor`) (`self.Mesh`) (`self.RightHandMeleeWeaponSocket`) "SnapToTarget" "SnapToTarget" "SnapToTarget" true)
          (set `self.IsWieldingWeapon` true))))))

(event `Start Block`
  (`MovementComponent.StopMovementImmediately` (`self.CharacterMovement`))
  (set `/Game/Blueprints/DamageSystem/BPC_DamageSystem.IsBlocking` true (`self.BPC_DamageSystem`))
  (set `self.BlockingState` "NewEnumerator1")
  (`|PlayMontage` (`self.Mesh`) (`self.MeleeBlockMontage`)
    (:`OnCompleted`
      (`self.EndBlock` :!label _label_2))
    (:`OnInterrupted`
      (if (`|EnumInequality` (`self.BlockingState`) "NewEnumerator2")
        (goto _label_2)))))

(event `self.BPC_DamageSystem.OnBlocked`
  (params (CanBeParried :type Boolean))
  (set `self.BlockingState` "NewEnumerator2")
  (bind _notifyname (`|PlayMontage` (`self.Mesh`) (`self.MeleeBlockMontageHit`))
    (:`OnCompleted`
      (`self.EndBlock` :!label _label_3))
    (:`OnInterrupted`
      (goto _label_3))
    (:`OnNotifyBegin`
      (switch `name` _notifyname
        (:`BlockStart`
          (`AkGameplayStatics.PostEvent` "/Game/WwiseAudio/Events/SFX/Enemy_Block.Enemy_Block" (`GameplayStatics.GetPlayerPawn` 0)))))))

(event `EndBlock`
  (set `/Game/Blueprints/DamageSystem/BPC_DamageSystem.IsBlocking` false (`self.BPC_DamageSystem`))
  (set `self.BlockingState` "NewEnumerator0")
  (`self.OnBlockEnded`))

(fn `GetIdealRange`
  (returns (AttackRadius :type "Float (double-precision)") (DefendRadius :type "Float (double-precision)"))
  (return 300.0 500.0))

(fn `UserConstructionScript`
  (`parent.UserConstructionScript`))