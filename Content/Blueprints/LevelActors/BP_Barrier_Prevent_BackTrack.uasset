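; BP_Barrier_Prevent_BackTrack is a level barrier that, going by its name, blocks players from backtracking between waves.
; On BeginPlay it caches the transform of its BarrierParent actor and binds to the wave-start event of BP_SpawnManager.
; When a wave starts and BarrierParent is no longer valid, it moves itself to the cached transform, taking that actor's place.
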(event `self.ReceiveBeginPlay`
  (bind _returnvalue (`GameplayStatics.GetActorOfClass` "/Game/Blueprints/LevelActors/BP_SpawnManager.BP_SpawnManager_C"))
  (add `/Game/Blueprints/LevelActors/BP_SpawnManager.OnWaveStart` _returnvalue (`|CreateDelegate` :!event `HandleOnWaveStart`))
  (set `self.BarrierParentTransform` (`self.GetTransform` (`self.BarrierParent`))))

(event `HandleOnWaveStart`
  (bind (_barrierparenttransform_location _barrierparenttransform_rotation _barrierparenttransform_scale) (`KismetMathLibrary.BreakTransform` (`self.BarrierParentTransform`)))
  (if (not (`KismetSystemLibrary.IsValid` (`self.BarrierParent`)))
    (`self.K2_SetActorTransform` (`KismetMathLibrary.MakeTransform` _barrierparenttransform_location _barrierparenttransform_rotation _barrierparenttransform_scale))))

(fn `UserConstructionScript`)