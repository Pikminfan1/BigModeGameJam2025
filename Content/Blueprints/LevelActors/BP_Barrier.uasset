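; BP_Barrier is a level barrier that breaks apart when its assigned area is cleared.
; On BeginPlay it binds to the OnAreaClear event of the BP_SpawnManager found in the level.
; When the cleared area matches AreaToClear, it swaps its mesh for a spawned BP_Fractured_Barrier at the same transform.
; It turns on physics for the fractured mesh, pushes it with a forward-vector force, then destroys itself after a short delay.
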(event `HandleAreaClear`
  (params (AreaCleared :type "/Game/Blueprints/LevelActors/E_Area Enum" :default "NewEnumerator0"))
  (bind _barriermesh (`self.BarrierMesh`))
  (if (`|EnumEquality` AreaCleared (`self.AreaToClear`))
    (bind _output_get (set `self.SpawnLocation` (`SceneComponent.K2_GetComponentToWorld` _barriermesh)))
    (`ActorComponent.K2_DestroyComponent` _barriermesh)
    (bind _returnvalue (`|SpawnActorFromClass` "/Game/Blueprints/LevelActors/BP_Fractured_Barrier.BP_Fractured_Barrier_C" (`KismetMathLibrary.MakeTransform` (.location _output_get) (.rotation _output_get)) "Undefined" "MultiplyWithRoot" null null))
    (bind _fracturedmesh (`/Game/Blueprints/LevelActors/BP_Fractured_Barrier.FracturedMesh` _returnvalue))
    (`PrimitiveComponent.SetSimulatePhysics` _fracturedmesh true)
    (`PrimitiveComponent.AddForceAtLocationLocal` _fracturedmesh (* (`self.GetActorForwardVector`) 100000.0) (0.0 0.0 0.0) "None")
    (`KismetSystemLibrary.Delay` 0.2)
    (`self.K2_DestroyActor`)))

(event `self.ReceiveActorBeginOverlap`
  (params (OtherActor :type "Actor Object Reference")))

(event `self.ReceiveBeginPlay`
  (bind _returnvalue (`GameplayStatics.GetActorOfClass` "/Game/Blueprints/LevelActors/BP_SpawnManager.BP_SpawnManager_C"))
  (`/Engine/EditorBlueprintResources/StandardMacros.IsValid` _returnvalue
    (:`Is Valid`
      (add `/Game/Blueprints/LevelActors/BP_SpawnManager.OnAreaClear` _returnvalue (delegate `HandleAreaClear`)))
    (:`Is Not Valid`
      (`KismetSystemLibrary.PrintString` "No spawn manager"))))

(fn `UserConstructionScript`)