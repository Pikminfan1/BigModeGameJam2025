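; BP_Fractured_Barrier is a fractured barrier level actor that removes itself after a set time.
; On BeginPlay it waits for LifeTime, then destroys itself.
; An area-clear handler is empty, and the nodes to bind it to BP_SpawnManager and raise the barrier when its area clears are disconnected, so they never run.
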(event `self.ReceiveBeginPlay`
  (`KismetSystemLibrary.Delay` (`self.LifeTime`))
  (`self.K2_DestroyActor`))

(event `HandleAreaClear`
  (params (AreaCleared :type "/Game/Blueprints/LevelActors/E_Area Enum" :default "NewEnumerator0")))

(fn `UserConstructionScript`)