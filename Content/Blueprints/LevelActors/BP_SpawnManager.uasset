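; Level actor that runs area-by-area enemy waves across five zones, from crypt to church.
; On BeginPlay it sorts every BP_Spawner by area and binds to spawner and player area trigger events.
; BeginNextArea starts a looping timer that spawns from that area's pool while active enemies stay under MaxEnemies.
; An area is clear when none are active or left to spawn, ending the wave; enemy deaths can broadcast OnAreaClear.
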(event `self.ReceiveBeginPlay`
  (`KismetSystemLibrary.Delay` 0.2)
  (`|ExecutionSequence`
    (:`then_0`
      (bind _outactors (`GameplayStatics.GetAllActorsOfClass` "/Game/Blueprints/LevelActors/BP_Spawner.BP_Spawner_C"))
      (for _array_element _outactors
        ; Add all spawners in level to a map organized by their location
        ;; Assign Spawners to groups
        (add `/Game/Blueprints/LevelActors/BP_Spawner.OnEnemySpawn` _array_element (`|CreateDelegate` :!event `HandleEnemySpawn`))
        (add `/Game/Blueprints/LevelActors/BP_Spawner.OnEnemyDeath_Spawner` _array_element (`|CreateDelegate` :!event `HandleEnemyDied`))
        (switch `/Game/Blueprints/LevelActors/E_Area` (`/Game/Blueprints/LevelActors/BP_Spawner.SpawnerArea` _array_element)
          (:`NewEnumerator1`
            (`KismetArrayLibrary.Array_Add` (`self.CryptSpawners`) _array_element))
          (:`NewEnumerator2`
            (`KismetArrayLibrary.Array_Add` (`self.TombSpawners`) _array_element))
          (:`NewEnumerator3`
            (`KismetArrayLibrary.Array_Add` (`self.GraveYardSpawners`) _array_element))
          (:`NewEnumerator4`
            (`KismetArrayLibrary.Array_Add` (`self.PathToChurchSpawners`) _array_element))
          (:`NewEnumerator5`
            (`KismetArrayLibrary.Array_Add` (`self.ChurchSpawners`) _array_element))))
      (bind _asbp_hybrid_character (cast `/Game/HybridPlayerController/BP_HybridCharacter` (`GameplayStatics.GetPlayerCharacter` 0)))
      (set `self.Hybrid Character Ref` _asbp_hybrid_character))
    (:`then_1`
      (bind _outactors_2 (`GameplayStatics.GetAllActorsOfClass` "/Game/Blueprints/LevelActors/BP_Player_Area_Trigger.BP_Player_Area_Trigger_C"))
      (for _array_element_2 _outactors_2
        (add `/Game/Blueprints/LevelActors/BP_Player_Area_Trigger.OnAreaSet` _array_element_2 (`|CreateDelegate` :!event `BeginNextArea`))))
    (:`then_2`
      (bind _asbp_big_mode_game_jam_2025game_mode (cast `/Game/Blueprints/BP_BigModeGameJam2025GameMode` (`GameplayStatics.GetGameMode`)))
      (set `self.Gamemode_Ref` _asbp_big_mode_game_jam_2025game_mode))))

(event `EnemyDied`
  (params (EnemyActor :type "Actor Object Reference") (NewParam :type "/Game/Blueprints/LevelActors/E_Area Enum" :default "NewEnumerator0")))

(event `Spawn Enemy`
  (params (AreaToSpawnIn :type "/Game/Blueprints/LevelActors/E_Area Enum" :default "NewEnumerator0"))
  (switch `/Game/Blueprints/LevelActors/E_Area` (`self.CurrentArea`)))

(event `HandleEnemyDied`
  (bind _areaisclear (`self.Get Is Area Clear` (`self.CurrentArea`)))
  (if _areaisclear
    (`self.OnAreaClear` (`self.CurrentArea`))))

(event `HandleEnemySpawn`
  (`/Engine/EditorBlueprintResources/StandardMacros.IncrementInt` (`self.CurrentEnemiesRemaining`)))

(event `BeginNextArea`
  (params (NewAreaSet :type "/Game/Blueprints/LevelActors/E_Area Enum" :default "NewEnumerator0"))
  (`KismetSystemLibrary.PrintString` "Next Area Reaching Starting area")
  (switch `/Game/Blueprints/LevelActors/E_Area` NewAreaSet
    (:`NewEnumerator1`
      (set `self.CurrentArea` "NewEnumerator1"))
    (:`NewEnumerator2`
      (set `self.CurrentArea` "NewEnumerator2"))
    (:`NewEnumerator3`
      (set `self.CurrentArea` "NewEnumerator3"))
    (:`NewEnumerator4`
      (set `self.CurrentArea` "NewEnumerator4"))
    (:`NewEnumerator5`
      (set `self.CurrentArea` "NewEnumerator5")))
  (`self.BeginSpawnWave`))

(event `BeginSpawnWave`
  (bind _returnvalue (`KismetSystemLibrary.K2_SetTimerDelegate` (delegate `OngoingWave`) 1.0 true))
  (set `self.CurrentWaveSpawnTimerHandle` _returnvalue))

(event `OngoingWave`
  (bind _areaisclear (`self.Get Is Area Clear` (`self.CurrentArea`)))
  (if _areaisclear
    (`self.EndWave`)
    (`KismetSystemLibrary.PrintString` "Wave end")
    (else
      (`KismetSystemLibrary.PrintString` "Wave ongoing")
      (switch `/Game/Blueprints/LevelActors/E_Area` (`self.CurrentArea`)
        (:`NewEnumerator1`
          (`self.HandleWave` (`self.CryptSpawners`)))
        (:`NewEnumerator2`
          (`self.HandleWave` (`self.TombSpawners`)))
        (:`NewEnumerator3`
          (`self.HandleWave` (`self.GraveYardSpawners`)))
        (:`NewEnumerator4`
          (`self.HandleWave` (`self.PathToChurchSpawners`)))
        (:`NewEnumerator5`
          (`self.HandleWave` (`self.ChurchSpawners`)))
        (:`NewEnumerator6`
          (`self.CountAllEnemies`))))))

(event `EndWave`
  (`KismetSystemLibrary.K2_ClearAndInvalidateTimerHandle` (`self.CurrentWaveSpawnTimerHandle`)))

(fn `CountAllEnemies`
  (returns (TotalEnemyCount :type Integer))
  (locals (TotalEnemies :type Integer))
  (set `local.TotalEnemies` 0)
  (bind _totalenemycount (`self.Get Enemies From Area` "NewEnumerator1"))
  (set `local.TotalEnemies` (+ _totalenemycount (`local.TotalEnemies`)))
  (bind _totalenemycount_2 (`self.Get Enemies From Area` "NewEnumerator2"))
  (set `local.TotalEnemies` (+ _totalenemycount_2 (`local.TotalEnemies`)))
  (bind _totalenemycount_3 (`self.Get Enemies From Area` "NewEnumerator3"))
  (set `local.TotalEnemies` (+ _totalenemycount_3 (`local.TotalEnemies`)))
  (bind _totalenemycount_4 (`self.Get Enemies From Area` "NewEnumerator4"))
  (set `local.TotalEnemies` (+ _totalenemycount_4 (`local.TotalEnemies`)))
  (bind _totalenemycount_5 (`self.Get Enemies From Area` "NewEnumerator5"))
  (bind _output_get (set `local.TotalEnemies` (+ _totalenemycount_5 (`local.TotalEnemies`))))
  (return _output_get))

(fn `Get Active Enemies From Area`
  (params (AreaToCountFrom :type "/Game/Blueprints/LevelActors/E_Area Enum" :default "NewEnumerator0"))
  (returns (TotalEnemyCount :type Integer))
  (locals (EnemyTotal :type Integer))
  (set `local.EnemyTotal` 0)
  (switch `/Game/Blueprints/LevelActors/E_Area` AreaToCountFrom
    (:`NewEnumerator1`
      (for _array_element (`self.CryptSpawners`)
        (set `local.EnemyTotal` (+ (`local.EnemyTotal`) (`/Game/Blueprints/LevelActors/BP_Spawner.ActiveEnemies` _array_element)))))
    (:`NewEnumerator2`
      (for _array_element_2 (`self.TombSpawners`)
        (set `local.EnemyTotal` (+ (`/Game/Blueprints/LevelActors/BP_Spawner.ActiveEnemies` _array_element_2) (`local.EnemyTotal`)))))
    (:`NewEnumerator3`
      (for _array_element_3 (`self.GraveYardSpawners`)
        (set `local.EnemyTotal` (+ (`local.EnemyTotal`) (`/Game/Blueprints/LevelActors/BP_Spawner.ActiveEnemies` _array_element_3)))))
    (:`NewEnumerator4`
      (for _array_element_4 (`self.PathToChurchSpawners`)
        (set `local.EnemyTotal` (+ (`local.EnemyTotal`) (`/Game/Blueprints/LevelActors/BP_Spawner.ActiveEnemies` _array_element_4)))))
    (:`NewEnumerator5`
      (for _array_element_5 (`self.ChurchSpawners`)
        (set `local.EnemyTotal` (+ (`local.EnemyTotal`) (`/Game/Blueprints/LevelActors/BP_Spawner.ActiveEnemies` _array_element_5))))))
  (return (`local.EnemyTotal`)))

(fn `Get Enemies From Area`
  (params (AreaToCountFrom :type "/Game/Blueprints/LevelActors/E_Area Enum" :default "NewEnumerator0"))
  (returns (TotalEnemyCount :type Integer))
  (locals (EnemyTotal :type Integer))
  (set `local.EnemyTotal` 0)
  (switch `/Game/Blueprints/LevelActors/E_Area` AreaToCountFrom
    (:`NewEnumerator1`
      (for _array_element (`self.CryptSpawners`)
        (bind _totalspawnableenemies (`/Game/Blueprints/LevelActors/BPI_Spawner.GetTotalEnemiesSpawnable` _array_element))
        (set `local.EnemyTotal` (+ (`local.EnemyTotal`) _totalspawnableenemies))))
    (:`NewEnumerator2`
      (for _array_element_2 (`self.TombSpawners`)
        (bind _totalspawnableenemies_2 (`/Game/Blueprints/LevelActors/BPI_Spawner.GetTotalEnemiesSpawnable` _array_element_2))
        (set `local.EnemyTotal` (+ _totalspawnableenemies_2 (`local.EnemyTotal`)))))
    (:`NewEnumerator3`
      (for _array_element_3 (`self.GraveYardSpawners`)
        (bind _totalspawnableenemies_3 (`/Game/Blueprints/LevelActors/BPI_Spawner.GetTotalEnemiesSpawnable` _array_element_3))
        (set `local.EnemyTotal` (+ (`local.EnemyTotal`) _totalspawnableenemies_3))))
    (:`NewEnumerator4`
      (for _array_element_4 (`self.PathToChurchSpawners`)
        (bind _totalspawnableenemies_4 (`/Game/Blueprints/LevelActors/BPI_Spawner.GetTotalEnemiesSpawnable` _array_element_4))
        (set `local.EnemyTotal` (+ (`local.EnemyTotal`) _totalspawnableenemies_4))))
    (:`NewEnumerator5`
      (for _array_element_5 (`self.ChurchSpawners`)
        (bind _totalspawnableenemies_5 (`/Game/Blueprints/LevelActors/BPI_Spawner.GetTotalEnemiesSpawnable` _array_element_5))
        (set `local.EnemyTotal` (+ (`local.EnemyTotal`) _totalspawnableenemies_5)))))
  (return (`local.EnemyTotal`)))

(fn `Get Is Area Clear`
  (params (Area :type "/Game/Blueprints/LevelActors/E_Area Enum" :default "NewEnumerator0"))
  (returns (AreaIsClear :type Boolean))
  (bind _totalenemycount (`self.GetEnemiesRemainingToSpawnInArea` Area))
  (bind _totalenemycount_2 (`self.Get Active Enemies From Area` Area))
  (if (== 0 _totalenemycount_2)
    (if (== _totalenemycount 0)
      (return true)
      (else
        (return false)))
    (else
      (return false))))

(fn `GetEnemiesRemainingToSpawnInArea`
  (params (Area :type "/Game/Blueprints/LevelActors/E_Area Enum" :default "NewEnumerator0"))
  (returns (TotalEnemyCount :type Integer))
  (locals (`Enemy Total` :type Integer))
  (set `local.Enemy Total` 0)
  (switch `/Game/Blueprints/LevelActors/E_Area` Area
    (:`NewEnumerator1`
      (for _array_element (`self.CryptSpawners`)
        (bind _enemy_count (`/Game/Blueprints/LevelActors/BPI_Spawner.GetEnemiesRemainingToSpawn` _array_element))
        (set `local.Enemy Total` (+ (`local.Enemy Total`) _enemy_count))))
    (:`NewEnumerator2`
      (for _array_element_2 (`self.TombSpawners`)
        (bind _enemy_count_2 (`/Game/Blueprints/LevelActors/BPI_Spawner.GetEnemiesRemainingToSpawn` _array_element_2))
        (set `local.Enemy Total` (+ (`local.Enemy Total`) _enemy_count_2))))
    (:`NewEnumerator3`
      (for _array_element_3 (`self.GraveYardSpawners`)
        (bind _enemy_count_3 (`/Game/Blueprints/LevelActors/BPI_Spawner.GetEnemiesRemainingToSpawn` _array_element_3))
        (set `local.Enemy Total` (+ (`local.Enemy Total`) _enemy_count_3))))
    (:`NewEnumerator4`
      (for _array_element_4 (`self.PathToChurchSpawners`)
        (bind _enemy_count_4 (`/Game/Blueprints/LevelActors/BPI_Spawner.GetEnemiesRemainingToSpawn` _array_element_4))
        (set `local.Enemy Total` (+ (`local.Enemy Total`) _enemy_count_4))))
    (:`NewEnumerator5`
      (for _array_element_5 (`self.ChurchSpawners`)
        (bind _enemy_count_5 (`/Game/Blueprints/LevelActors/BPI_Spawner.GetEnemiesRemainingToSpawn` _array_element_5))
        (set `local.Enemy Total` (+ (`local.Enemy Total`) _enemy_count_5)))))
  (return (`local.Enemy Total`)))

(fn `HandleWave`
  (params (PoolOfSpawners :type "Array of /Game/Blueprints/LevelActors/BP_Spawner Object Reference"))
  ; For each spawner, check if it can spawn, and spawn if max enemies isnt reached
  (for _array_element PoolOfSpawners
    (`KismetSystemLibrary.PrintString` (`KismetSystemLibrary.GetDisplayName` _array_element))
    (if (`/Game/Blueprints/LevelActors/BP_Spawner.CanSpawn` _array_element)
      (bind _totalenemycount (`self.Get Active Enemies From Area` (`self.CurrentArea`)))
      (if (< _totalenemycount (`self.MaxEnemies`))
        (bind _enemy_data_to_spawn (`/Game/Blueprints/LevelActors/BP_Spawner.SelectEnemyToSpawn` _array_element))
        (`/Game/Blueprints/LevelActors/BP_Spawner.Spawn Enemy` _array_element _enemy_data_to_spawn)
        (else
          (`KismetSystemLibrary.PrintString` "Cant spawn, is max enemies reached?"))))))

(fn `Set Current Area`
  (params (CurrentArea :type "/Game/Blueprints/LevelActors/E_Area Enum" :default "NewEnumerator0"))
  (returns (NewArea :type "/Game/Blueprints/LevelActors/E_Area Enum"))
  (switch `/Game/Blueprints/LevelActors/E_Area` CurrentArea
    (:`NewEnumerator0`
      (set `self.CurrentArea` "NewEnumerator1")
      (return "NewEnumerator0"))
    (:`NewEnumerator1`
      (set `self.CurrentArea` "NewEnumerator2"))
    (:`NewEnumerator2`
      (set `self.CurrentArea` "NewEnumerator3"))
    (:`NewEnumerator3`
      (set `self.CurrentArea` "NewEnumerator4"))
    (:`NewEnumerator4`
      (set `self.CurrentArea` "NewEnumerator5"))
    (:`NewEnumerator5`
      (set `self.CurrentArea` "NewEnumerator6"))))

(fn `SetMaxEnemies`
  (switch `/Game/Blueprints/LevelActors/E_Difficulty` (`/Game/Blueprints/BP_BigModeGameJam2025GameMode.CurrentDifficulty` (`self.Gamemode_Ref`))
    (:`NewEnumerator0`
      (set `self.MaxEnemies` 5))
    (:`NewEnumerator1`
      (set `self.MaxEnemies` 10))
    (:`NewEnumerator2`
      (set `self.MaxEnemies` 15))
    (:`NewEnumerator3`
      (set `self.MaxEnemies` 20))))

(fn `SpawnEnemyCheck`
  (if (`|EnumEquality` (`self.CurrentArea`) (`self.CurrentArea`))
    (`KismetSystemLibrary.PrintString` "Spawn Manager")))

(fn `UserConstructionScript`)