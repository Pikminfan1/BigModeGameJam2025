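; Revolver projectile Blueprint that damages whatever it hits and then destroys itself.
; On hit, it sends an interrupting damage struct through a TakeDamage interface message and reports the damage event for AI perception.
; BeginPlay runs the parent logic and sets the skeletal mesh play rate, while the projectile impact handler only prints the hit actor's name.
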(event `self.ReceiveBeginPlay`
  (`parent.ReceiveBeginPlay`)
  (`SkeletalMeshComponent.SetPlayRate` (`self.SkeletalMesh`) 1.0))

(event `self.ReceiveActorBeginOverlap`
  (params (OtherActor :type "Actor Object Reference")))

(event `self.ReceiveHit`
  (params (MyComp :type "PrimitiveComponent Object Reference") (Other :type "Actor Object Reference") (OtherComp :type "PrimitiveComponent Object Reference") (bSelfMoved :type Boolean) (HitLocation :type "Vector Structure") (HitNormal :type "Vector Structure") (NormalImpulse :type "Vector Structure") (Hit :type "HitResult Structure (by ref)"))
  (bind _instigator (`self.Instigator`))
  (bind _damage (`self.Damage`))
  (message `/Game/Blueprints/DamageSystem/BPI_Damagable.TakeDamageActor` Other (make `/Game/Blueprints/DamageSystem/S_DamageInfo` _damage "NewEnumerator2" "NewEnumerator0" false false false true) _instigator (`self.HitResult`))
  (`AISense_Damage.ReportDamageEvent` Other _instigator _damage HitLocation)
  (`self.K2_DestroyActor`))

(event `OnProjectileImpact_Event`
  (params (OtherActor :type "Actor Object Reference") (Hit :type "HitResult Structure"))
  (`KismetSystemLibrary.PrintString` (`KismetSystemLibrary.GetDisplayName` OtherActor)))

(fn `UserConstructionScript`
  (`parent.UserConstructionScript`))