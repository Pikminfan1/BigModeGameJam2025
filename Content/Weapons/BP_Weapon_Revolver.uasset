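; Revolver weapon Blueprint that tracks its own ammo and exposes a fire point.
; FireShot removes one round, clamped between zero and MaxAmmo, and returns whether the count actually changed.
; Reload refills to MaxAmmo, and simple getters report fire point, ammo, capacity and empty state.
; The event graph holds no active logic, and FireShot handles only the ammo count, with no projectile, trace or effects.
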(fn `FireShot`
  (returns (FireShotSuccess :type Boolean))
  (locals (AmmoBeforeShot :type "Float (double-precision)"))
  ; Tell me if we actually depleted ammo
  (set `local.AmmoBeforeShot` (`self.Ammo`))
  (set `self.Ammo` (`KismetMathLibrary.FClamp` (- (`self.Ammo`) 1.0) 0.0 (`self.MaxAmmo`)))
  (if (== (`local.AmmoBeforeShot`) (`self.Ammo`))
    (return false)
    (else
      (return true))))

(fn `GetAmmo`
  (returns (Ammo :type "Float (double-precision)"))
  (return (`self.Ammo`)))

(fn `GetFirePoint`
  (returns (FirePoint :type "SceneComponent Object Reference"))
  (return (`self.FirePoint`)))

(fn `GetMaxAmmo`
  (returns (MaxAmmo :type "Float (double-precision)"))
  (return (`self.MaxAmmo`)))

(fn `IsEmpty`
  (returns (IsEmpty :type Boolean))
  (return (<= (`self.Ammo`) 0.0)))

(fn `Reload`
  (set `self.Ammo` (`self.MaxAmmo`)))

(fn `UserConstructionScript`
  (`parent.UserConstructionScript`))